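; In-game player controller that links the possessed character to team NPCs, saved settings and voice commands.
; On server possession it tags the pawn defender (local player 0) or attacker and initializes matching NPC controllers with that character.
; The replicated Controlling flag's RepNotify passes saved formations and dimensions to the character for the server.
; Speech setup spawns a keyword recognizer for fixed and saved-formation phrases, forwarding spoken text as character command requests.
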(event `sendDimensionsToServer`
  (bind _settingssaveobject (`SiegeGameInstance.settingsSaveObject` (cast `SiegeGameInstance` (`GameplayStatics.GetGameInstance`) :!pure true)))
  (bind _asthird_person_character (cast `/Game/ThirdPersonCPP/Blueprints/ThirdPersonCharacter` (`self.K2_GetPawn`)))
  (`/Engine/EditorBlueprintResources/StandardMacros.IsValid` _settingssaveobject
    (:`Is Valid`
      (`/Game/ThirdPersonCPP/Blueprints/ThirdPersonCharacter.recieveDimensions` _asthird_person_character (`SettingsSave.dimensions` _settingssaveobject)))))

(event `send_formations_to_server`
  (bind _formationsaveobject (`SiegeGameInstance.formationSaveObject` (cast `SiegeGameInstance` (`GameplayStatics.GetGameInstance`) :!pure true)))
  (bind _asthird_person_character (cast `/Game/ThirdPersonCPP/Blueprints/ThirdPersonCharacter` (`self.K2_GetPawn`)))
  (`/Engine/EditorBlueprintResources/StandardMacros.IsValid` _formationsaveobject
    (:`Is Valid`
      (`/Game/ThirdPersonCPP/Blueprints/ThirdPersonCharacter.recieve_formations` _asthird_person_character (`FormationSaveGame.formationsSaved` _formationsaveobject))
      (`KismetSystemLibrary.PrintString` "formations send"))))

(event `self.ReceivePossess`
  (params (PossessedPawn :type "Pawn Object Reference"))
  (bind _tags (`Actor.Tags` (`self.K2_GetPawn`)))
  (if (`KismetSystemLibrary.IsServer`)
    (set `self.controlling` true)
    (if (== (`GameplayStatics.GetPlayerController` 0) self)
      (set `Actor.Tags` (`|MakeArray` "player" "defender" :!type "Name") (`self.K2_GetPawn`))
      (else
        (set `Actor.Tags` (`|MakeArray` "player" "attacker" :!type "Name") (`self.K2_GetPawn`))))
    (if (`KismetArrayLibrary.Array_IsValidIndex` _tags 1)
      (bind _outactors (`GameplayStatics.GetAllActorsOfClassWithTag` "/Game/npc/npc.npc_C" (`|GetArrayItem` _tags 1)))
      (for _array_element _outactors
        (bind _asnpccontroller (cast `/Game/npc/npccontroller` (`AIBlueprintHelperLibrary.GetAIController` _array_element)))
        (`/Game/npc/npccontroller.initalize` _asnpccontroller (cast `/Game/ThirdPersonCPP/Blueprints/ThirdPersonCharacter` (`self.K2_GetPawn`) :!pure true))))))

(event `setupspeech`
  (bind _speechactor (`self.speechactor`))
  (bind _speechactor_2 (`self.Speechactor`))
  (bind _formationsaveobject (`SiegeGameInstance.formationSaveObject` (cast `SiegeGameInstance` (`GameplayStatics.GetGameInstance`) :!pure true)))
  (bind _returnvalue (`|SpawnActorFromClass` "/Script/SpeechRecognition.SpeechRecognitionActor" (`KismetMathLibrary.MakeTransform` (0.0 0.0 0.0)) "AlwaysSpawn" "OverrideRootScale" null null))
  (set `self.speechactor` _returnvalue)
  (bind _returnvalue_2 (`SpeechRecognitionActor.Init` _speechactor "VE_English"))
  (if _returnvalue_2
    (`KismetSystemLibrary.PrintString` "did speech setup")
    (`SpeechRecognitionActor.SetConfigParam` _speechactor "-vad_prespeech" "VE_INTEGER" "10")
    (`SpeechRecognitionActor.SetConfigParam` _speechactor "-vad_postspeech" "VE_INTEGER" "10")
    (`SpeechRecognitionActor.SetConfigParam` _speechactor "-agc" "VE_STRING" "noise")
    (`SpeechRecognitionActor.SetConfigParam` _speechactor "-beam" "VE_FLOAT" "1e-40")
    (set `self.commands` (`|MakeArray` (make `RecognitionPhrase` "follow me" "VE_6") (make `RecognitionPhrase` "attack" "VE_7") (make `RecognitionPhrase` "attention" "VE_7") (make `RecognitionPhrase` "fall in" "VE_5") (make `RecognitionPhrase` "dismissed" "VE_7")))
    (`/Engine/EditorBlueprintResources/StandardMacros.IsValid` _formationsaveobject
      (:`Is Valid`
        (for _array_element (`FormationSaveGame.formationsSaved` _formationsaveobject)
          (`KismetArrayLibrary.Array_Append` (`self.commands`) (`|MakeArray` (make `RecognitionPhrase` (`KismetStringLibrary.Concat_StrStr` "formation " (`.name` (break `FormationStruct` _array_element))))))))
      (:`Is Not Valid`
        _))
    (if true
      (`SpeechRecognitionActor.EnableKeywordMode` _speechactor_2 (`self.commands`))
      (add `SpeechRecognitionActor.OnWordsSpoken` _speechactor_2 (delegate `onspoken`)))))

(event `self.ReceiveEndPlay`
  (params (EndPlayReason :type "EEndPlayReason Enum" :default "Destroyed"))
  (bind _speechactor (`self.speechactor`))
  (`/Engine/EditorBlueprintResources/StandardMacros.IsValid` _speechactor
    (:`Is Valid`
      (`SpeechRecognitionActor.Shutdown` _speechactor))))

(event `onspoken`
  (params (Text :type "RecognisedPhrases Structure"))
  (bind _asthird_person_character (cast `/Game/ThirdPersonCPP/Blueprints/ThirdPersonCharacter` (`GameplayStatics.GetPlayerCharacter` 0)))
  (`/Game/ThirdPersonCPP/Blueprints/ThirdPersonCharacter.requestcommand` _asthird_person_character Text))

(fn `OnRep_controlling`
  (if (`self.controlling`)
    (`self.send_formations_to_server`)
    (`self.sendDimensionsToServer`)))

(fn `UserConstructionScript`)